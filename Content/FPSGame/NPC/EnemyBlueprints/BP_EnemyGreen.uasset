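; BP_EnemyGreen is an enemy NPC that moves toward the player when detected and reacts to damage.
; LookForLight repeats a delayed forward box trace from the head, moving to the hit component on BP_Player and resuming only if that move succeeds.
; HealthComponent receives damage, triggering a random hit-react section with a brief movement stop, and ragdolls the enemy on death before removal.
; Most other interface functions, such as healing, weapon and patrol, are empty stubs.
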(event OnDeath(HealthComponent)
  (Utilities|FlowControl|DoOnce false
    (:Completed
      (Collision|SetCollisionProfileName (Variables|Character|GetMesh) "Ragdoll" true :!class /Script/Engine.PrimitiveComponent)
      (Class|SkeletalMeshComponent|SetAllBodiesSimulatePhysics (Variables|Character|GetMesh) true)
      (Collision|SetCollisionEnabled (Variables|Collision|GetCapsuleComponent) "NoCollision")
      (Actor|SetLifeSpan 6.0))))

(event OnDamageTaken(HealthComponent)
  (bind _charactermovement (Variables|Character|GetCharacterMovement))
  (Variables|Default|SettempSpeed (Variables|/Script/Engine.CharacterMovementComponent|GetMaxWalkSpeed _charactermovement))
  (Variables|/Script/Engine.CharacterMovementComponent|SetMaxWalkSpeed _charactermovement 0.0)
  (Animation|PlayAnimMontage "/Game/FPSGame/NPC/EnemyMeshes/EnemyGreen/AnimationsFromMixamo/GreenE_HitReact.GreenE_HitReact" 1.4 (Utilities|String|StringToName (Utilities|String|ToString(Integer) (Math|Random|RandomIntegerinRange 1 2))))
  (Utilities|FlowControl|Delay 0.2)
  (Variables|/Script/Engine.CharacterMovementComponent|SetMaxWalkSpeed _charactermovement (Variables|Default|GettempSpeed)))

(event Custom|LookForLight
  (bind _mesh (Variables|Character|GetMesh))
  (bind _returnvalue (Transformation|GetSocketLocation _mesh "HeadSocket"))
  (Utilities|FlowControl|Delay 0.5)
  (bind (_outhit _returnvalue_2) (Collision|BoxTraceByChannel _returnvalue (+ _returnvalue (* (Math|Vector|GetForwardVector (Transformation|GetActorRotation)) 1.2e+03)) "70.000000,70.000000,50.000000" "0, 0, 0" "TraceTypeQuery2" false 0 "None" true "(R=1.000000,G=0.000000,B=0.000000,A=1.000000)" "(R=0.000000,G=1.000000,B=0.000000,A=1.000000)" 1.0))
  (if _returnvalue_2
    (Utilities|Casting|CastToBP_Player (.HitActor (Collision|BreakHitResult _outhit))
      (:then
        (AI|AIMoveTo 0 (Transformation|GetWorldLocation (.HitComponent (Collision|BreakHitResult _outhit))) 0 5.0 false
          (:OnSuccess
            _)))
      (:CastFailed
        _)))
  (CallFunction|LookforLight))

(event EventBeginPlay
  (CallFunction|LookforLight))

(event EventNotifyStateChanged
  (params (NewState :type NPCState%20Enum :default "NewEnumerator0"))
  ;[0.2675 0.1551 0.2865] On State Changed
  (Class|BPIAIHelper|NotifyStateChanged(Message) (Components|SkeletalMesh|GetAnimInstance (Variables|Character|GetMesh)) NewState))

(fn ConstructionScript)

(fn UpdateWalkSpeed
  (params (NewWalkSpeed :type Float%20%28single-precision%29))
  (Variables|/Script/Engine.CharacterMovementComponent|SetMaxWalkSpeed (Variables|Character|GetCharacterMovement) NewWalkSpeed))

(fn GetCurrentHealthBPID
  (return 0.0))

(fn GetIsDead
  (return (Default|IsDead? (Variables|Default|GetHealthComponent))))

(fn GetMaxHealthBPID
  (return 0.0))

(fn GetPatrolRoute
  (return 0))

(fn GetTeamID
  (return false))

(fn GetWeapon
  (return false 0))

(fn GetWeaponRange
  (return 0.0))

(fn HealBPID
  (params (Amount :type Float%20%28single-precision%29))
  (return 0.0))

(fn IsDeadBPID
  (return false))

(fn TakeDamageBPID
  (params (DamageInfo :type S%20Damage%20Info%20Structure))
  (bind _healthcomponent (Variables|Default|GetHealthComponent))
  (Default|TakeDamageHC _healthcomponent DamageInfo)
  (Default|CallOnDamageTaken _healthcomponent)
  (Development|PrintString (Utilities|String|ToString(Float) (Variables|/Game/FPSGame/Blueprints/DamageSystemDG/HealthComponent.HealthComponent_C|GetHealth _healthcomponent)))
  (return false))