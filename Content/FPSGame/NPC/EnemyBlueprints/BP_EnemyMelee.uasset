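; Melee enemy NPC that carries a sword, attacks with a montage combo and blocks hits.
; It spawns the sword on BeginPlay, then equip and unequip montages use notifies to move it between sheath and hand sockets.
; Attacks disable interruption on the HealthComponent, while blocking sets its block flag and plays an impact montage when a hit is blocked.
; Montage endings fire dispatchers for equip, attack and block, with block end feeding the Behavior Tree.
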(event OnBlocked(HealthComponent)
  (params (CanBeParried :type Boolean))
  (Variables|Default|SetBlockingState "NewEnumerator1")
  (Animation|Montage|PlayMontage (Variables|Character|GetMesh) "/Game/FPSGame/NPC/EnemyMeshes/EnemyBase/Animations/Montages/Montage_Great_Sword_Impact.Montage_Great_Sword_Impact"
    (:OnCompleted
      _)
    (:OnInterrupted
      _))
  (CallFunction|EndBlock))

(event Custom|StartBlock
  (Variables|/Game/FPSGame/Blueprints/DamageSystemDG/HealthComponent.HealthComponent_C|SetIsBlocking (Variables|Default|GetHealthComponent) true)
  (Variables|Default|SetBlockingState "NewEnumerator1")
  (Animation|Montage|PlayMontage (Variables|Character|GetMesh) "/Game/FPSGame/NPC/EnemyMeshes/EnemyBase/Animations/Montages/Montage_Great_Sword_Blocking.Montage_Great_Sword_Blocking"
    (:OnCompleted
      (CallFunction|EndBlock :!label _label))
    (:OnInterrupted
      (if (Utilities|Enum|NotEqual(Enum) (Variables|Default|GetBlockingState) "NewEnumerator2")
        (goto _label)))))

(event Custom|EndBlock
  (Variables|/Game/FPSGame/Blueprints/DamageSystemDG/HealthComponent.HealthComponent_C|SetIsBlocking (Variables|Default|GetHealthComponent) false)
  (Variables|Default|SetBlockingState "NewEnumerator0")
  ;[0.04504 0.1562 0.0405] event dispatch created and called from here which is accessed in the BT
  (Default|CallOnBlockEnded))

(event EventBeginPlay
  (|CallParentFunction)
  (bind _returnvalue (Game|SpawnActorfromClass "/Game/FPSGame/NPC/EnemyWeapons/BP_WeaponSword.BP_WeaponSword_C" (Transformation|GetActorTransform) "Undefined" 0 0))
  (bind _output_get (Variables|Default|SetWeaponActor _returnvalue))
  (Transformation|AttachComponentToComponent _output_get (Variables|Character|GetMesh) "SwordSheathSocket" "SnapToTarget" "SnapToTarget" "SnapToTarget" true))

(event EventUnEquipWeapon
  (bind _notifyname (Animation|Montage|PlayMontage (Variables|Character|GetMesh) "/Game/FPSGame/NPC/EnemyMeshes/EnemyBase/Animations/Montages/Sword_Sheath_Montage.Sword_Sheath_Montage")
    (:OnCompleted
      (Default|CallOnWeaponUnEquipped))
    (:OnNotifyBegin
      (switch name _notifyname
        (:SheathSword
          (Variables|Default|SetIsWeildingweapon false)
          (Transformation|AttachComponentToComponent (Variables|Default|GetWeaponActor) (Variables|Character|GetMesh) "SwordSheathSocket" "SnapToTarget" "SnapToTarget" "SnapToTarget" true))))))

(event EventEquipWeapon
  (bind _notifyname (Animation|Montage|PlayMontage (Variables|Character|GetMesh) "/Game/FPSGame/NPC/EnemyMeshes/EnemyBase/Animations/Montages/Sword_Weild_Montage.Sword_Weild_Montage")
    (:OnCompleted
      (Default|CallOnWeaponEquipped))
    (:OnNotifyBegin
      (switch name _notifyname
        (:WithdrawSword
          (Transformation|AttachComponentToComponent (Variables|Default|GetWeaponActor) (Variables|Character|GetMesh) "SwordSocket" "SnapToTarget" "SnapToTarget" "SnapToTarget" true)
          (Variables|Default|SetIsWeildingweapon true))))))

(event EventAttack
  (Animation|Montage|PlayMontage (Variables|Character|GetMesh) "/Game/FPSGame/NPC/EnemyMeshes/EnemyBase/Animations/Montages/Sowrd_Attack_Combo_CL_Heavy_Montage.Sowrd_Attack_Combo_CL_Heavy_Montage"
    (:then
      ;[0.1583 0.2917 0.04237] Can't be interrupted if atrtacking
      (Variables|/Game/FPSGame/Blueprints/DamageSystemDG/HealthComponent.HealthComponent_C|SetIsInterruptable (Variables|Default|GetHealthComponent) false))
    (:OnCompleted
      (Default|CallOnAttackEnd :!label _label) ; event dispatched only when animation is completed or interrupted.
      (Variables|/Game/FPSGame/Blueprints/DamageSystemDG/HealthComponent.HealthComponent_C|SetIsInterruptable (Variables|Default|GetHealthComponent) true))
    (:OnInterrupted
      (goto _label))))

(fn ConstructionScript
  (|CallParentFunction))