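; Health component that tracks an actor's health, healing and death in the damage system.
; TakeDamageHC filters damage through a CanBeDamaged macro for invincibility and blocking, then fires dispatchers for blocks, hit responses or death.
; Self-calling, Delay-paced events provide gradual drain and regeneration, the latter only above a health threshold.
; The older OnTakeAnyDamage route that triggered draining is disconnected.
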(event Custom|OnTakeAnyDamage
  (params (DamagedActor :type Actor%20Object%20Reference) (Damage :type Float%20%28single-precision%29) (DamageType :type Damage%20Type%20Object%20Reference) (InstigatedBy :type Controller%20Object%20Reference) (DamageCauser :type Actor%20Object%20Reference)))

(event Custom|DepreciateHealth
  ;[1 0.2499 0.5909] Depreciate Health
  (if (Variables|Default|GetShouldDrain?)
    (if (<= (Math|Float|Clamp(Float) (- (Variables|Default|GetHealth) (Variables|Default|GetHealthReductionSpeed)) 0.0 (Variables|Default|GetMaxHealth)) 0.0)
      (Variables|Default|SetHealth 0.0)
      (Variables|Default|SetIsDead true)
      (else
        (Variables|Default|SetHealth (Math|Float|Clamp(Float) (- (Variables|Default|GetHealth) (Variables|Default|GetHealthReductionSpeed)) 0.0 (Variables|Default|GetMaxHealth)))
        (bind _output_get (Variables|Default|SetEnemyDamage (Math|Float|Clamp(Float) (- (Variables|Default|GetEnemyDamage) (Variables|Default|GetHealthReductionSpeed)) 0.0 (Variables|Default|GetMaxHealth))))
        (if (<= _output_get 0.0)
          (Variables|Default|SetShouldDrain? false)
          (Variables|Default|SetEnemyDamage 0.0)
          (else
            (Utilities|FlowControl|Delay 0.001)
            (CallFunction|DepreciateHealth)))))))

(event Custom|AppreciateHealth
  ;[1 0.2499 0.5909] Appreciate Health- Health will increase only if Health is greater than 30 and is not equal to MaxHealth
  (if (not (or (CallFunction|IsDead?) (Variables|Default|GetIsDead)))
    (if (not (Variables|Default|GetShouldDrain?))
      (bind _appreciatehealth_ (CallFunction|AppreciateHealth?))
      (if _appreciatehealth_
        (bind _newhealth (CallFunction|IncreaseHealth))
        (Variables|Default|SetHealth _newhealth)
        (Utilities|FlowControl|Delay 0.08)
        (CallFunction|AppreciateHealth)))))

(event EventBeginPlay
  (Variables|Default|SetHealth (Variables|Default|GetMaxHealth)))

(fn IsDead?
  (return (<= (Variables|Default|GetHealth) 0.0)))

(fn Heal
  (params (Amount :type Float%20%28single-precision%29))
  (if (not (Variables|Default|GetIsDead))
    (bind _output_get (Variables|Default|SetHealth (Math|Float|Clamp(Float) (+ Amount (Variables|Default|GetHealth)) 0.0 (Variables|Default|GetMaxHealth))))
    (return _output_get)))

(fn TakeDamageHC
  (params (DamageInfo :type S%20Damage%20Info%20Structure) (DamageCauser :type Actor%20Object%20Reference))
  (bind (_amount _damagetype _damageresponse _shoulddamageinvincible _canbeblocked _canbeparried _shouldforceinterrupt) (Utilities|Struct|BreakS_DamageInfo DamageInfo))
  (Utilities|CanbeDamaged _shoulddamageinvincible _canbeblocked
    (:BlockDamage
      (Default|CallOnBlocked _canbeparried)
      (return false))
    (:DoDamage
      (bind _output_get (Variables|Default|SetHealth (- (Variables|Default|GetHealth) _amount)))
      (if (<= _output_get 0.0)
        (Variables|Default|SetIsDead true)
        (Default|CallOnDeath)
        (return true)
        (elif (or (Variables|Default|GetIsInterruptable) _shouldforceinterrupt)
          (Default|CallOnDamageResponse _damageresponse DamageCauser)
          (return true))))
    (:NoDamage
      (return false))))

(fn AppreciateHealth?
  (return (and (!= (Variables|Default|GetHealth) (Variables|Default|GetMaxHealth)) (> (Variables|Default|GetHealth) 3e+01))))

(fn IncreaseHealth
  (return (Math|Float|Clamp(Float) (+ (Variables|Default|GetHealth) (Variables|Default|GetHealthAppreciateAmount)) 0.0 (Variables|Default|GetMaxHealth))))